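; BP_player is a side-scrolling 2D player character that runs along the world X axis and jumps, animated with sprite flipbooks.
; Axis input drives movement, and the jump action starts and stops jumping and sets the jump-up flipbook.
; Each tick selects the falling, run or idle flipbook from movement state, which can immediately replace jump-up.
; Tick also flips control yaw to face the X velocity direction.
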(event `self.ReceiveTick`
  (params (DeltaSeconds :type "Float (single-precision)"))
  (`self.movement_update`)
  (`self.rotation_update`))

(event `InputAxis|movement`
  (params (AxisValue :type "Float (single-precision)"))
  (`self.AddMovementInput` (1.0 0.0 0.0) AxisValue))

(event `movement_update`
  (`PaperFlipbookComponent.SetFlipbook` (`self.Sprite`) (select `bool` (`NavMovementComponent.IsFalling` (`self.CharacterMovement`)) :`false` (select `bool` (> (`KismetMathLibrary.VSize` (`MovementComponent.Velocity` (`self.CharacterMovement`))) 0.0) :`false` "/Game/Assets/sprites/png/idle/FB_idle.FB_idle" :`true` "/Game/Assets/sprites/png/run/FB_run.FB_run" :!type "PaperFlipbook Object Reference") :`true` "/Game/Assets/sprites/png/jump/FB_jump_fall.FB_jump_fall")))

(event `rotation_update`
  (bind _velocity_x (`KismetMathLibrary.BreakVector` (`MovementComponent.Velocity` (`self.CharacterMovement`))))
  (`/Engine/EditorBlueprintResources/StandardMacros.IsValid` (`self.GetController`)
    (:`Is Valid`
      (`/Engine/EditorBlueprintResources/StandardMacros.CompareFloat` _velocity_x
        (:`>`
          (`Controller.SetControlRotation` (`self.GetController`) (`KismetMathLibrary.MakeRotator` 0.0)))
        (:`<`
          (`Controller.SetControlRotation` (`self.GetController`) (`KismetMathLibrary.MakeRotator` 0.0 0.0 180.0)))))))

(event `InputAction|jump`
  (params (Key :type "Key Structure"))
  (:`Pressed`
    (`self.Jump`)
    (`PaperFlipbookComponent.SetFlipbook` (`self.Sprite`) "/Game/Assets/sprites/png/jump/FB_jump_up.FB_jump_up"))
  (:`Released`
    (`self.StopJumping`)))

(fn `UserConstructionScript`)